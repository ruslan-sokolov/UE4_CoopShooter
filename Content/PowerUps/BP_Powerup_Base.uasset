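; Base Blueprint for powerups that animates a pickup mesh and handles the feedback for activation and expiry.
; Each tick spins the mesh by a period-scaled rotation and moves it back and forth, inverting its velocity whenever the period elapses.
; Activation hides the mesh and plays a pickup sound, while deactivation shows it and plays a powerdown sound.
; On expiry, the actor destroys itself after a brief delay.
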(event `self.ReceiveTick`
  (params (DeltaSeconds :type "Float (single-precision)"))
  (`self.RotateMeshWithPeriod` DeltaSeconds)
  (`self.MoveMeshWithPeriod` DeltaSeconds))

(event `self.OnExpired`
  (`KismetSystemLibrary.Delay` 0.1)
  (`self.K2_DestroyActor`))

(event `self.OnPowerupStateChanged`
  (params (bNewIsActive :type Boolean))
  (`SceneComponent.SetVisibility` (`self.StaticMesh`) (not bNewIsActive) true)
  (if bNewIsActive
    (`GameplayStatics.PlaySound2D` "/Game/PowerUps/Assets/Pickup_powerup.Pickup_powerup" 1.0 1.0 0.0 null null)
    (else
      (`GameplayStatics.PlaySound2D` "/Game/PowerUps/Assets/powerdown_02.powerdown_02" 1.0 1.0 0.0 null null))))

(fn `MoveMeshWithPeriod`
  (params (DeltaTime :type "Float (double-precision)"))
  (locals (DeltaVelocity :type "Vector Structure"))
  (bind _output_get (set `self.MoveDuration` (+ DeltaTime (`self.MoveDuration`))))
  (`|ExecutionSequence`
    (:`then_0`
      (if (>= _output_get (`self.Period`))
        (set `self.MoveDuration` 0.0)
        (set `self.bInvertMoveVelocity` (not (`self.bInvertMoveVelocity`)))))
    (:`then_1`
      (if (`self.bInvertMoveVelocity`)
        (set `local.DeltaVelocity` (* (`self.MoveVelocity`) (* (`local.DeltaTime`) -1.0)))
        (else
          (set `local.DeltaVelocity` (* (`self.MoveVelocity`) (`local.DeltaTime`)))))
      (`SceneComponent.K2_AddWorldOffset` (`self.StaticMesh`) (`local.DeltaVelocity`) false false))))

(fn `RotateMeshWithPeriod`
  (params (DeltaTime :type "Float (double-precision)"))
  (`SceneComponent.K2_AddWorldRotation` (`self.StaticMesh`) (* (`self.Rotator`) (/ DeltaTime (`self.Period`))) false false))

(fn `UserConstructionScript`)