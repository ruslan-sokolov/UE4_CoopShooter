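; Player character Blueprint that adds a health indicator and a temporary gun cheat menu for the locally controlled player.
; Q toggles the menu, and while it is open keys 1-3 call SpawnWeapon for rifle, grenade launcher or pistol.
; Health changes draw the delta as debug text at the actor, and the construction script attaches the spring arm to the mesh's spine_03 socket.
; Leftover test snippets sit unconnected in the event graph.
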(event `Key|E`
  (params (Key :type "Key Structure"))
  ;[1 1 1] test balls
)

(event `self.ReceiveBeginPlay`
  (if (`self.IsLocallyControlled`)
    (`|ExecutionSequence`
      (:`then_0`
        ;[1 1 1] Temp gun cheat menu
        (bind _returnvalue (`|CreateWidget` "/Game/UI/WBP_GunCheats.WBP_GunCheats_C"))
        (bind _output_get (set `self.WBP_GUN_MENU_TEMP` _returnvalue))
        (`UserWidget.AddToViewport` _output_get 0))
      (:`then_1`
        (bind _returnvalue_2 (`|CreateWidget` "/Game/UI/WBP_HealthIndicator.WBP_HealthIndicator_C"))
        (`UserWidget.AddToViewport` _returnvalue_2 0)))))

(event `Key|One`
  (params (Key :type "Key Structure"))
  ;[1 1 1] Temp Gun Cheat Menu Control
  (:`Pressed`
    (if (`self.GunMenuIsOpen`)
      (`self.SpawnWeapon` "/Game/Blueprints/BP_Rifle.BP_Rifle_C"))))

(event `Key|Two`
  (params (Key :type "Key Structure"))
  ;[1 1 1] Temp Gun Cheat Menu Control
  (:`Pressed`
    (if (`self.GunMenuIsOpen`)
      (`self.SpawnWeapon` "/Game/Blueprints/BP_GranadeLauncher.BP_GranadeLauncher_C"))))

(event `Key|Three`
  (params (Key :type "Key Structure"))
  ;[1 1 1] Temp Gun Cheat Menu Control
  (:`Pressed`
    (if (`self.GunMenuIsOpen`)
      (`self.SpawnWeapon` "/Game/Blueprints/BP_Pistol.BP_Pistol_C"))))

(event `Key|Q`
  (params (Key :type "Key Structure"))
  (bind _wbp_gun_menu_temp (`self.WBP_GUN_MENU_TEMP`))
  (bind _returnvalue (`KismetSystemLibrary.IsValid` (`self.WBP_GUN_MENU_TEMP`)))
  ;[1 1 1] Temp Gun Cheat Menu Control
  (:`Pressed`
    (`/Engine/EditorBlueprintResources/StandardMacros.FlipFlop`
      (:`A`
        (if _returnvalue
          (`/Game/UI/WBP_GunCheats.OpenMenu` _wbp_gun_menu_temp)
          (set `self.GunMenuIsOpen` true)))
      (:`B`
        (if _returnvalue
          (`/Game/UI/WBP_GunCheats.CloseMenu` _wbp_gun_menu_temp)
          (set `self.GunMenuIsOpen` false))))))

(event `self.HealthComp.OnHealthChanged`
  (params (HealthComp :type "SHealthComponent Object Reference") (Health :type "Float (single-precision)") (HealthDelta :type "Float (single-precision)") (DamageType :type "DamageType Object Reference") (InstigatedBy :type "Controller Object Reference") (DamageCauser :type "Actor Object Reference"))
  (`KismetSystemLibrary.DrawDebugString` (`self.K2_GetActorLocation`) (`KismetStringLibrary.Conv_DoubleToString` HealthDelta) null (struct :`R` 1.0 :`A` 1.0) 1.0))

(event `self.ReceiveTick`
  (params (DeltaSeconds :type "Float (single-precision)")))

(fn `UserConstructionScript`
  (`SceneComponent.K2_AttachToComponent` (`self.SpringArmComp`) (`self.Mesh`) "spine_03" "KeepRelative" "KeepRelative" "KeepRelative" true))