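; BP_TestBall is a physics test ball that launches upward to a target height, comparing two launch methods.
; ActivateAction either sets linear velocity (labeled force) or adds a velocity-change impulse, both using sqrt(2gh) from CalcVerticalForceToReachZ.
; Tick times upward movement and draws mass, height and that time at the ball, with text and material colored by method.
; A gated AddForce branch is disconnected.
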(event `ActivateAction`
  (if (`self.UseForceInsteadOfImpulse`)
    (`self.AddForceOnDemand`)
    (else
      (`self.AddImpulseOnDemand`))))

(event `AddForceOnDemand`
  ;[1 0.9 0.09166] force
  (`PrimitiveComponent.SetPhysicsLinearVelocity` (`self.StaticMesh`) (`self.CalcVerticalForceToReachZ` 4000.0) false "None"))

(event `AddImpulseOnDemand`
  ;[0 0.7699 1] impulse
  (`PrimitiveComponent.AddImpulse` (`self.StaticMesh`) (`self.CalcVerticalForceToReachZ` 4000.0) "None" true))

(event `ChangeMaterialColor`
  (bind _staticmesh (`self.StaticMesh`))
  (bind _returnvalue (`PrimitiveComponent.CreateDynamicMaterialInstance` _staticmesh 0 (`PrimitiveComponent.GetMaterial` _staticmesh 0) "None"))
  (bind _output_get (set `self.DynMaterial` _returnvalue))
  (`PrimitiveComponent.SetMaterial` (`self.StaticMesh`) 0 _output_get)
  (`MaterialInstanceDynamic.SetVectorParameterValue` (`self.DynMaterial`) "Color_1" (`KismetMathLibrary.Conv_ColorToLinearColor` (select `bool` (`self.UseForceInsteadOfImpulse`) :`false` (`self.ColorImpulse`) :`true` (`self.ColorForce`)))))

(event `self.ReceiveBeginPlay`
  (set `self.LastLocation` (`self.K2_GetActorLocation`))
  (`self.ChangeMaterialColor`)
  (`self.EnableInput` (`GameplayStatics.GetPlayerController` 0)))

(event `self.ReceiveTick`
  (params (DeltaSeconds :type "Float (single-precision)"))
  (`self.TimeMovingUpHandle` DeltaSeconds)
  (`self.PrintMessage` DeltaSeconds))

(fn `CalcVerticalForceToReachZ`
  (params (Z :type "Float (double-precision)"))
  (returns (VerticalForce :type "Vector Structure"))
  (bind _returnvalue (`KismetMathLibrary.Sqrt` (* Z 980.0 2.0)))
  (`KismetSystemLibrary.PrintString` (`KismetStringLibrary.Concat_StrStr` "Z velocity:" (`KismetStringLibrary.Conv_DoubleToString` _returnvalue) " t predict:" (`KismetStringLibrary.Conv_DoubleToString` (/ (* Z 2.0) _returnvalue))))
  (return (`KismetMathLibrary.MakeVector` 0.0 0.0 _returnvalue)))

(fn `PrintMessage`
  (params (DeltaSec :type "Float (double-precision)"))
  (bind _returnvalue (`self.K2_GetActorLocation`))
  (`KismetSystemLibrary.DrawDebugString` _returnvalue (`KismetStringLibrary.Concat_StrStr` "m: " (`KismetTextLibrary.Conv_TextToString` (`KismetTextLibrary.Conv_DoubleToText` (`PrimitiveComponent.GetMass` (`self.StaticMesh`)) "HalfToEven" false true 1 324 0 0)) "Z:" (`KismetTextLibrary.Conv_TextToString` (`KismetTextLibrary.Conv_DoubleToText` (.z _returnvalue) "HalfToEven" false true 1 324 0 0)) "t:" (`KismetTextLibrary.Conv_TextToString` (`KismetTextLibrary.Conv_DoubleToText` (`self.TimeMovingUp`) "HalfToEven" false true 1 324 1 1))) null (`KismetMathLibrary.Conv_ColorToLinearColor` (select `bool` (`self.UseForceInsteadOfImpulse`) :`false` (`self.ColorImpulse`) :`true` (`self.ColorForce`))) DeltaSec))

(fn `TimeMovingUpHandle`
  (params (DeltaSec :type "Float (double-precision)"))
  (bind (_returnvalue_x _returnvalue_y _returnvalue_z) (`KismetMathLibrary.BreakVector` (`self.K2_GetActorLocation`)))
  (bind (_lastlocation_x _lastlocation_y _lastlocation_z) (`KismetMathLibrary.BreakVector` (`self.LastLocation`)))
  (`|ExecutionSequence`
    (:`then_0`
      (if (> _returnvalue_z _lastlocation_z)
        ;[1 1 1] moving up
        (`|ExecutionSequence`
          (:`then_0`
            ;;[1 1 1] When start moving up again drop counter
            (if (`self.bLastMoveWasDown`)
              (set `self.bLastMoveWasDown` false)
              (set `self.TimeMovingUp` 0.0)))
          (:`then_1`
            ;;[1 1 1] append time in air moving up
            (set `self.TimeMovingUp` (+ (`self.TimeMovingUp`) (`local.DeltaSec`)))))
        (else
          ;[1 1 1] moving down
          (set `self.bLastMoveWasDown` true))))
    (:`then_1`
      ;[1 1 1] update last pos
      (set `self.LastLocation` (`self.K2_GetActorLocation`)))))

(fn `UserConstructionScript`)