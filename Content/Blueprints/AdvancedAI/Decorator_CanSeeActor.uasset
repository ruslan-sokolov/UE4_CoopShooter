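; Behavior Tree decorator that passes when the AI's pawn currently senses the actor stored in the ActorToCheck blackboard key.
; It looks up the AIPerceptionComponent on the controlled pawn rather than the controller and queries that actor's perception info.
; The result is the successfully-sensed flag of the first last-sensed stimulus, with no check of which sense produced it.
; A missing component or perception record fails the condition.
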(fn `PerformConditionCheckAI`
  (params (OwnerController :type "AIController Object Reference") (ControlledPawn :type "Pawn Object Reference"))
  (returns (ReturnValue :type Boolean))
  (bind _returnvalue (`Actor.GetComponentByClass` ControlledPawn "/Script/AIModule.AIPerceptionComponent"))
  (`/Engine/EditorBlueprintResources/StandardMacros.IsValid` _returnvalue
    (:`Is Valid`
      (bind (_info _returnvalue_2) (`AIPerceptionComponent.GetActorsPerception` _returnvalue (`BTFunctionLibrary.GetBlackboardValueAsActor` (`self.ActorToCheck`))))
      (if _returnvalue_2
        (return (`.bSuccessfullySensed` (break `AIStimulus` (`|GetArrayItem` (`.LastSensedStimuli` (break `ActorPerceptionBlueprintInfo` _info))))))
        (else
          _)))
    (:`Is Not Valid`
      _))
  (return false))