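; Advanced AI pawn that starts the BT_AdvancedAI behavior tree on its AI controller at BeginPlay.
; Its HealingComponent start and end events drive heal feedback: an attached spark emitter and sound are spawned, then destroyed, with one-shot cues at each transition.
; Weapon no-ammo debug logging and a deprecated Blackboard target hack remain in the graph but are not wired to run.
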(event `self.ReceiveBeginPlay`
  (bind _returnvalue (`AIBlueprintHelperLibrary.GetAIController` self))
  (`/Engine/EditorBlueprintResources/StandardMacros.IsValid` self
    (:`Is Valid`
      (`/Engine/EditorBlueprintResources/StandardMacros.IsValid` _returnvalue
        (:`Is Valid`
          (`AIController.RunBehaviorTree` _returnvalue "/Game/Blueprints/AdvancedAI/BT_AdvancedAI.BT_AdvancedAI"))))))

(event `OnCharacterWeaponSpawned_Event_0` :!signature `self.OnCharacterWeaponSpawned`
  (params (Character :type "SCharacter Object Reference") (Weapon :type "SWeapon Object Reference"))
  ;[1 1 1] no ammo left event
  (add `SWeapon.OnNoAmmoLeft` Weapon (delegate `OnNoAmmoLeft_Event_0`)))

(event `OnNoAmmoLeft_Event_0`
  (params (Weapon :type "SWeapon Object Reference"))
  ;[1 1 1] no ammo left event
  (`KismetSystemLibrary.PrintString` (`KismetStringLibrary.Concat_StrStr` (`KismetSystemLibrary.GetObjectName` self) " Has no ammo in " (`KismetSystemLibrary.GetObjectName` Weapon))))

(event `self.HealingComponent.OnActorHealStart`
  (params (HealActor :type "Actor Object Reference") (HealthBefore :type "Float (single-precision)"))
  (`self.StartHealFXEvent`))

(event `self.HealingComponent.OnActorHealEnd`
  (params (HealActor :type "Actor Object Reference") (HealthAfter :type "Float (single-precision)") (Success :type Boolean))
  (`self.EndHealFXEvent`))

(event `StartHealFXEvent`
  (bind _mesh (`self.Mesh`))
  (`|ExecutionSequence`
    (:`then_0`
      (`GameplayStatics.PlaySoundAtLocation` "/Game/Blueprints/AI/DroneTracker_idle.DroneTracker_idle" (`self.K2_GetActorLocation`) (struct) 1.0 1.0 0.0 null null null)
      (bind _returnvalue (`GameplayStatics.SpawnEmitterAttached` "/Game/StarterContent/Particles/P_Sparks.P_Sparks" _mesh "neck_01" (0.0 0.0 -15.0) (struct) (1.0 1.0 1.0) "KeepRelativeOffset" false "None" false))
      (bind _output_get (set `self.HealEmitter` _returnvalue))
      (if (`KismetSystemLibrary.IsValid` _output_get)
        (`ActorComponent.Activate` _output_get false)))
    (:`then_1`
      (bind _returnvalue_2 (`GameplayStatics.SpawnSoundAttached` "/Game/StarterContent/Audio/Fire_Sparks01_Cue1.Fire_Sparks01_Cue1" _mesh "spine_03" (0.0 0.0 15.0) (struct) "KeepRelativeOffset" false 1.0 1.0 0.0 null null))
      (bind _output_get_2 (set `self.HealSound` _returnvalue_2))
      (if (`KismetSystemLibrary.IsValid` _output_get_2)
        (`ActorComponent.Activate` _output_get_2 false)
        (`AudioComponent.Play` _output_get_2 0.0)))))

(event `EndHealFXEvent`
  (bind _healsound (`self.HealSound`))
  (bind _healemitter (`self.HealEmitter`))
  (`|ExecutionSequence`
    (:`then_0`
      (`/Engine/EditorBlueprintResources/StandardMacros.IsValid` _healemitter
        (:`Is Valid`
          (`ActorComponent.K2_DestroyComponent` _healemitter))))
    (:`then_1`
      (`/Engine/EditorBlueprintResources/StandardMacros.IsValid` _healsound
        (:`Is Valid`
          (`AudioComponent.Stop` _healsound)
          (`ActorComponent.K2_DestroyComponent` _healsound))))
    (:`then_2`
      (`GameplayStatics.PlaySoundAtLocation` "/Game/Blueprints/AI/DroneTracker_explodewarning.DroneTracker_explodewarning" (`self.K2_GetActorLocation`) (struct) 1.0 1.0 0.0 null null null))))

(fn `EndHealFX`)

(fn `UserConstructionScript`)