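; Co-op wave game mode that spawns tracker bots and awards score for kills.
; SpawnNewBot runs an EQS query (random best 25%), then spawns BP_TrackerBot at the resulting locations with debug spheres and wave logging.
; BeginPlay binds OnActorKilled, which adds fixed points to the killer's CoopPlayerState when the victim pawn is not player-controlled, and prints the kill.
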(event `self.SpawnNewBot`
  (bind _returnvalue (`EnvQueryManager.RunEQSQuery` "/Game/Blueprints/GameMode/Navigation/EQS_FindSpawnLocation.EQS_FindSpawnLocation" self "RandomBest25Pct"))
  (add `EnvQueryInstanceBlueprintWrapper.OnQueryFinishedEvent` _returnvalue (delegate `OnQueryFinished_SpawnBot`)))

(event `OnQueryFinished_SpawnBot`
  (params (QueryInstance :type "EnvQueryInstanceBlueprintWrapper Object Reference") (QueryStatus :type "EEnvQueryStatus Enum" :default "Processing"))
  ;[1 1 1] Spawn TrackerBot Using EQS System
  (switch `EEnvQueryStatus` QueryStatus
    (:`Success`
      (bind _resultlocations (`EnvQueryInstanceBlueprintWrapper.GetQueryResultsAsLocations` QueryInstance))
      (for _array_element _resultlocations
        (`KismetSystemLibrary.DrawDebugSphere` _array_element 50.0 12 (struct :`R` 1.0 :`G` 0.924858 :`A` 1.0) 2.0 2.0)
        (bind _returnvalue (`|SpawnActorFromClass` "/Game/Blueprints/AI/BP_TrackerBot.BP_TrackerBot_C" (`KismetMathLibrary.MakeTransform` _array_element) "AdjustIfPossibleButDontSpawnIfColliding" "OverrideRootScale" null null))
        (`KismetSystemLibrary.PrintString` (`KismetStringLibrary.Concat_StrStr` "[GameMode] " (`KismetSystemLibrary.GetDisplayName` _returnvalue) " spawned." " Current Wave: " (`KismetStringLibrary.Conv_IntToString` (`self.WaveCount`)) " Wave spawn left: " (`KismetStringLibrary.Conv_IntToString` (`self.NrOfBotsToSpawn`))) true true (struct :`R` 1.0 :`G` 1.0 :`A` 1.0))))))

(event `self.ReceiveBeginPlay`
  (add `self.OnActorKilled` (delegate `OnActorKilled_Event_0`)))

(event `OnActorKilled_Event_0` :!signature `self.OnActorKilled`
  (params (VictimActor :type "Actor Object Reference") (KillerActor :type "Actor Object Reference") (KillerController :type "Controller Object Reference"))
  (bind _returnvalue (`Controller.K2_GetPawn` KillerController))
  ;[0.3854 0.3854 0.3854] on !(player controlled) pawn killed add score event
  ;;[1 1 1] victim not player controlled
  (bind _aspawn (cast `Pawn` VictimActor))
  (if (not (`Pawn.IsPlayerControlled` _aspawn))
    ;;[1 1 1] Killer add score
    (`/Engine/EditorBlueprintResources/StandardMacros.IsValid` _returnvalue
      (:`Is Valid`
        (bind _ascoop_player_state (cast `CoopPlayerState` (`Pawn.PlayerState` _returnvalue)))
        (`CoopPlayerState.AddScore` _ascoop_player_state 20.0)
        (`KismetSystemLibrary.PrintString` (`KismetStringLibrary.Concat_StrStr` (`KismetSystemLibrary.GetObjectName` VictimActor) " killed by" (`KismetSystemLibrary.GetObjectName` _returnvalue) " using " (`KismetSystemLibrary.GetObjectName` KillerActor) ". Total score: " (`KismetStringLibrary.Conv_DoubleToString` (`PlayerState.Score` _ascoop_player_state)) ".") true true (struct :`R` 0.66 :`G` 1.0 :`A` 1.0) 4.0)))))

(fn `UserConstructionScript`)